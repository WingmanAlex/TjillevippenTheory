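; Trigger actor that changes the player character's scale each time it overlaps the Changer component.
; A selector picks the small, large or normal scale, then advances modulo three to cycle through them.
; A Gate closes right after each change and reopens after a one-second Delay, so overlaps during that cooldown are ignored.
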(event OnComponentBeginOverlap(Changer)
  (params (OverlappedComponent :type Primitive%20Component%20Object%20Reference) (OtherActor :type Actor%20Object%20Reference) (OtherComp :type Primitive%20Component%20Object%20Reference) (OtherBodyIndex :type Integer) (bFromSweep :type Boolean) (SweepResult :type Hit%20Result%20Structure%20%28by%20ref%29))
  (bind _returnvalue (Game|GetPlayerCharacter 0))
  (if (== _returnvalue OtherActor)
    (Utilities|FlowControl|Sequence
      (:then_0
        (Utilities|FlowControl|Gate false :!label _label
          (:Exit
            (Transformation|SetActorScale3D _returnvalue (Math|Conversions|ToVector(Float) (Utilities|Select :Index (Variables|Default|GetSelector) :Option%200 (Variables|Default|GetScaleSmall) :Option%201 (Variables|Default|GetScale%20Large) :Option%202 (Variables|Default|GetScale%20Normal))))
            (bind _result (Math|Integer|IncrementInt (Variables|Default|GetSelector))
              (:%20%20
                (Variables|Default|SetSelector (Math|Integer|%(Integer) _result 3))
                (Utilities|FlowControl|Delay 1.0)
                (goto _label Open))))))
      (:then_1
        (goto _label Close)))))

(fn ConstructionScript)